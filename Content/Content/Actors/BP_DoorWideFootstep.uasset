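; Interactable wide door with footstep that the player opens and closes with the Interact input.
; A trigger overlap shows a HUD prompt built from the bound key, enables input and opens a gate.
; Interact either plays the open animation or closes by negating its play rate, tracked by DoorOpen.
; Leaving hides the prompt, disables input and reverses the play rate, leaving DoorOpen and the gate untouched.
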(event OnComponentBeginOverlap(Trigger)
  (params (OverlappedComponent :type Primitive%20Component%20Object%20Reference) (OtherActor :type Actor%20Object%20Reference) (OtherComp :type Primitive%20Component%20Object%20Reference) (OtherBodyIndex :type Integer) (bFromSweep :type Boolean) (SweepResult :type Hit%20Result%20Structure%20%28by%20ref%29))
  (bind _asbp_princess_character (Utilities|Casting|CastToBP_Princess_Character OtherActor))
  (bind _asfirst_person_hud (Utilities|Casting|CastToFirstPersonHUD (Variables|/Script/Project_Princess.Project_PrincessCharacter|GetFPS_HUD_Ref _asbp_princess_character)))
  (if (Variables|Default|GetDoorOpen)
    (Variables|Default|SetOpenClose "Close")
    (else
      (Variables|Default|SetOpenClose "Open")))
  (bind _returnstring (CallFunction|SetInteractTxt (stale Input|ActionEvents|InputActionInteract Key) (Variables|Default|GetOpenClose)))
  (Default|ShowInteractText _asfirst_person_hud _returnstring)
  (Input|EnableInput (Game|GetPlayerController 0))
  (Utilities|FlowControl|Gate true) ; enters at Open
)

(event OnComponentEndOverlap(Trigger)
  (params (OverlappedComponent :type Primitive%20Component%20Object%20Reference) (OtherActor :type Actor%20Object%20Reference) (OtherComp :type Primitive%20Component%20Object%20Reference) (OtherBodyIndex :type Integer))
  (bind _asproject_princess_character (Utilities|Casting|CastToProject_PrincessCharacter OtherActor))
  (bind _asfirst_person_hud (Utilities|Casting|CastToFirstPersonHUD (Variables|/Script/Project_Princess.Project_PrincessCharacter|GetFPS_HUD_Ref _asproject_princess_character)))
  (Default|HideinteractText _asfirst_person_hud)
  (Input|DisableInput (Game|GetPlayerController 0))
  (CallFunction|ReverseAnimation))

(event EventBeginPlay)

(event Collision|EventActorBeginOverlap
  (params (OtherActor :type Actor%20Object%20Reference)))

(event EventTick
  (params (DeltaSeconds :type Float%20%28single-precision%29)))

(event Input|ActionEvents|InputActionInteract
  (params (Key :type Key%20Structure))
  (:Pressed
    (Utilities|FlowControl|Gate true
      (:Exit
        (if (Variables|Default|GetDoorOpen)
          (CallFunction|ReverseAnimation)
          (Variables|Default|SetDoorOpen false)
          (else
            (Components|Animation|PlayAnimation (Variables|Default|GetDoor_WideWithFootstep) "/Game/Content/Meshes/DoorWide_withFootstep/Door_WideWithFootstep_Anim.Door_WideWithFootstep_Anim" false)
            (Variables|Default|SetDoorOpen true)))))))

(event Input|KeyboardEvents|E
  (params (Key :type Key%20Structure)))

(fn ConstructionScript)

(fn ReverseAnimation
  (bind _door_widewithfootstep (Variables|Default|GetDoor_WideWithFootstep))
  (Components|Timeline|SetPlayRate _door_widewithfootstep (* (Components|Animation|GetPlayRate _door_widewithfootstep) -1.0)))

(fn SetInteractTxt
  (params (Key :type Key%20Structure) (OpenClose :type String))
  (bind _output_get (LocalVariables|SetOutputString (Utilities|Text|ToText(String) (Utilities|String|Append "Press \" " (Utilities|String|ToString(Text) (Class|KismetInputLibrary|KeyGetDisplayName (.Key (Utilities|Struct|BreakInputActionKeyMapping (Utilities|Array|Get(acopy) (Class|InputSettings|GetActionMappingbyName (Class|InputSettings|GetInputSettings) "Interact")))))) " \" to " OpenClose))))
  (Development|PrintString (Utilities|String|ToString(Text) _output_get) true true "(R=1.000000,G=0.000000,B=0.000000,A=1.000000)")
  (return (Utilities|String|ToString(Text) _output_get)))